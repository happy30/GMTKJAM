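; BaseItem is a collectible pickup, named as a base item, that spins steadily around its yaw axis on Tick.
; When a BP_FPSController overlaps it, it increments that actor's ItemsCollected and has FPSGameMode show a notification with the item name.
; If MakePlayerSick is set, it also resets the game mode's countdown for the next sneeze event, then destroys itself in either case.
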(event EventBeginPlay)

(event Collision|EventActorBeginOverlap
  (params (OtherActor :type Actor%20Object%20Reference))
  (bind _asbp_fpscontroller (Utilities|Casting|CastToBP_FPSController OtherActor))
  (Math|Integer|IncrementInt (Variables|/Game/Blueprints/BP_FPSController.BP_FPSController_C|GetItemsCollected _asbp_fpscontroller)
    (:%20%20
      (bind _asfpsgame_mode (Utilities|Casting|CastToFPSGameMode (Game|GetGameMode)))
      (Default|ShowItemNotification _asfpsgame_mode (Variables|Default|GetItemName))
      (if (Variables|Default|GetMakePlayerSick)
        (bind _asfpsgame_mode_2 (Utilities|Casting|CastToFPSGameMode (Game|GetGameMode)))
        (Default|ResetCountingforNextSneezeEvent _asfpsgame_mode_2))
      (Actor|DestroyActor))))

(event EventTick
  (params (DeltaSeconds :type Float%20%28single-precision%29))
  (Transformation|AddActorLocalRotation (* (Math|Rotator|MakeRotator 0.0 0.0 45.0) DeltaSeconds) false false))

(fn ConstructionScript)