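; ScuseMeGameInstance is the game instance that owns the persistent save object for the game.
; On Init it loads the "Save" slot and caches it as a ScuseMeSaveGame, or creates and immediately writes a new one if none loads.
; A failed cast only prints a debug string, leaving the reference unset.
; A Save event writes the cached object back to the same slot.
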(event Custom|Save
  (SaveGame|SaveGametoSlot (Variables|Default|GetSaveGame) "Save"))

(event EventInit
  (bind _returnvalue (SaveGame|LoadGamefromSlot "Save"))
  (Utilities|IsValid _returnvalue
    (:Is%20Valid
      (bind _asscuse_me_save_game (Utilities|Casting|CastToScuseMeSaveGame _returnvalue)
        (:then
          (Variables|Default|SetSaveGame _asscuse_me_save_game))
        (:CastFailed
          (Development|PrintString "Hello"))))
    (:Is%20Not%20Valid
      (bind _returnvalue_2 (SaveGame|CreateSaveGameObject "/Game/Blueprints/ScuseMeSaveGame.ScuseMeSaveGame_C"))
      (bind _output_get (Variables|Default|SetSaveGame _returnvalue_2))
      (SaveGame|SaveGametoSlot _output_get "Save"))))