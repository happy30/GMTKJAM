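; Level exit actor that ends the level when an overlapping BP_FPSController has collected enough items.
; On overlap it plays the FadeIn sequence in reverse and fades out all ambient sounds.
; When the sequence finishes, it plays a jingle, removes the damage fee widget, pauses the game and shows a Rating screen with cursor input.
; The rank comes from comparing the game mode's total damage cost against descending thresholds.
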(event Custom|NextLevel
  (bind _returnvalue (Game|GetPlayerController 0))
  (Audio|PlaySound2D "/Game/Sound/EndLevelJingle.EndLevelJingle" 1.0 1.0 0.0 0 0)
  (bind _asfpsgame_mode (Utilities|Casting|CastToFPSGameMode (Game|GetGameMode)))
  (Widget|RemovefromParent (Variables|/Game/Blueprints/FPSGameMode.FPSGameMode_C|GetDamageFee _asfpsgame_mode))
  (bind _rank (CallFunction|DetermineLevelRank (Variables|/Game/Blueprints/FPSGameMode.FPSGameMode_C|GetTotalDamageCost _asfpsgame_mode)))
  (bind _returnvalue_2 (UserInterface|CreateWidget "/Game/Blueprints/Rating.Rating_C"))
  (Default|Fillin _returnvalue_2 (Variables|Default|GetItemsNeeded) (Variables|/Game/Blueprints/FPSGameMode.FPSGameMode_C|GetTotalDamageCost _asfpsgame_mode) _rank "None" (Variables|Default|GetCurrentLevel))
  (UserInterface|Viewport|AddtoViewport _returnvalue_2 0)
  (Game|SetGamePaused true)
  (Input|SetInputModeUIOnly _returnvalue 0 "DoNotLock")
  (Variables|/Script/Engine.PlayerController|SetbShowMouseCursor _returnvalue true))

(event EventBeginPlay)

(event Collision|EventActorBeginOverlap
  (params (OtherActor :type Actor%20Object%20Reference))
  (bind _asbp_fpscontroller (Utilities|Casting|CastToBP_FPSController OtherActor))
  (if (>= (Variables|/Game/Blueprints/BP_FPSController.BP_FPSController_C|GetItemsCollected _asbp_fpscontroller) (Variables|Default|GetItemsNeeded))
    (bind _outactor (Sequencer|Player|CreateLevelSequencePlayer "/Game/Cinematics/FadeIn.FadeIn" (Utilities|Struct|MakeMovieSceneSequencePlaybackSettings false "(Value=0)" 1.0 0.0 false false false false false false false true)))
    (Class|MovieSceneSequencePlayer|PlayReverse (Variables|/Script/LevelSequence.LevelSequenceActor|GetSequencePlayer _outactor))
    (EventDispatchers|BindEventtoOnFinished (Variables|/Script/LevelSequence.LevelSequenceActor|GetSequencePlayer _outactor) (delegate Custom|NextLevel))
    (bind _outactors (Actor|GetAllActorsOfClass "/Script/Engine.AmbientSound"))
    (for _array_element _outactors
      (Audio|Components|Audio|FadeOut (Variables|/Script/Engine.AmbientSound|GetAudioComponent _array_element) 1.0 0.0 "Linear" :!class /Script/Engine.AudioComponent))))

(event EventTick
  (params (DeltaSeconds :type Float%20%28single-precision%29)))

(fn ConstructionScript)

(fn DetermineLevelRank
  (params (DamageDone :type Integer))
  (if (> DamageDone (Variables|Default|GetMaxDamageRankE))
    (return "NewEnumerator0")
    (elif (> DamageDone (Variables|Default|GetMaxDamageRankD))
      (return "NewEnumerator1")
      (elif (> DamageDone (Variables|Default|GetMaxDamageRankC))
        (return "NewEnumerator2")
        (elif (> DamageDone (Variables|Default|GetMaxDamageRankB))
          (return "NewEnumerator3")
          (elif (> DamageDone (Variables|Default|GetMaxDamageRankA))
            (return "NewEnumerator4")
            (elif (> DamageDone (Variables|Default|GetMaxDamageRankS))
              (return "NewEnumerator5")
              (elif (> DamageDone (Variables|Default|GetMaxDamageRankSS))
                (return "NewEnumerator6")
                (else
                  (return "NewEnumerator7"))))))))))