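; First-person player character controller with mouse look, movement, a cooldown-limited dash and a sneeze attack.
; Space starts an anticipation phase that shows a warning widget and shifts camera FOV until a timer fires the sneeze.
; The sneeze spawns a force impulse, hits overlapping NPCs, recoils the player and notifies FPSGameMode.
; Becoming sick resets the game mode's sneeze countdown, and Tick also handles dash recharge.
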(event EventBeginPlay
  (if (Variables|Default|GetIsSick)
    (bind _asfpsgame_mode (Utilities|Casting|CastToFPSGameMode (Game|GetGameMode)))
    (Default|ResetCountingforNextSneezeEvent _asfpsgame_mode)
    (Variables|Default|SetInitialFoV (Variables|/Script/Engine.CameraComponent|GetFieldOfView (Variables|Default|GetCamera)))))

(event Collision|EventActorBeginOverlap
  (params (OtherActor :type Actor%20Object%20Reference)))

(event EventTick
  (params (DeltaSeconds :type Float%20%28single-precision%29))
  (bind _camera (Variables|Default|GetCamera))
  (if (Variables|Default|GetAnticipatingSneeze)
    (if (< (Variables|Default|GetAnticipatingSneezeTimer) (Variables|Default|GetSneezeAnticipationTime))
      (Variables|Default|SetAnticipatingSneezeTimer (+ (Variables|Default|GetAnticipatingSneezeTimer) DeltaSeconds))
      (Camera|SetFieldOfView _camera (+ (* DeltaSeconds (Variables|Default|GetFoVChangeSpeed)) (Variables|/Script/Engine.CameraComponent|GetFieldOfView _camera)))
      (Variables|Default|SetMoveDirection (Math|Vector|MakeVector (stale Input|AxisEvents|InputAxisHorizontal AxisValue) (stale Input|AxisEvents|InputAxisVertical AxisValue) 0.0) :!label _label)
      (if (not (Variables|Default|GetCanDash))
        (Utilities|FlowControl|Delay (Variables|Default|GetDashCoolDown))
        (Variables|Default|SetCanDash true))
      (else
        (CallFunction|Sneeze)))
    (else
      (goto _label))))

(event Input|ActionEvents|InputActionDash
  (params (Key :type Key%20Structure))
  (:Pressed
    (if (Variables|Default|GetCanDash)
      (CallFunction|Dash)
      (Variables|Default|SetCanDash false))))

(event Input|AxisEvents|InputAxisMouseHorizontal
  (params (AxisValue :type Float%20%28single-precision%29))
  (Pawn|Input|AddControllerYawInput AxisValue))

(event Input|AxisEvents|InputAxisMouseVertical
  (params (AxisValue :type Float%20%28single-precision%29))
  (Pawn|Input|AddControllerPitchInput AxisValue))

(event Input|AxisEvents|InputAxisVertical
  (params (AxisValue :type Float%20%28single-precision%29))
  (Pawn|Input|AddMovementInput (Math|Vector|GetForwardVector (Math|Rotator|MakeRotator 0.0 0.0 (.yaw (Pawn|GetControlRotation :!class /Script/Engine.Pawn)))) AxisValue false))

(event Input|AxisEvents|InputAxisHorizontal
  (params (AxisValue :type Float%20%28single-precision%29))
  (Pawn|Input|AddMovementInput (Math|Vector|GetRightVector (Math|Rotator|MakeRotator 0.0 0.0 (.yaw (Pawn|GetControlRotation :!class /Script/Engine.Pawn)))) AxisValue false))

(event Input|KeyboardEvents|SpaceBar
  (params (Key :type Key%20Structure))
  (:Pressed
    (CallFunction|AnticipateSneeze)))

(fn ConstructionScript)

(fn Sneeze
  (bind _springarm (Variables|Default|GetSpringArm))
  (bind _returnvalue (Math|Vector|GetForwardVector _springarm))
  (bind _returnvalue_2 (* _returnvalue 1e+02))
  (bind (_x _y) (Math|Vector|BreakVector _returnvalue_2))
  (Variables|Default|SetAnticipatingSneeze false)
  (bind _returnvalue_3 (Game|SpawnActorfromClass "/Game/Blueprints/SneezeForce.SneezeForce_C" (Math|Transform|MakeTransform (+ (Transformation|GetActorLocation) _returnvalue_2)) "Undefined" 0 0))
  (Class|RadialForceComponent|FireImpulse (Variables|/Script/Engine.RadialForceActor|GetForceComponent _returnvalue_3))
  (Rendering|Debug|DrawDebugSphere (Transformation|GetWorldLocation (Variables|/Script/Engine.RadialForceActor|GetForceComponent _returnvalue_3)) (Variables|/Script/Engine.RadialForceComponent|GetRadius (Variables|/Script/Engine.RadialForceActor|GetForceComponent _returnvalue_3)) 12 "(R=1.000000,G=0.000000,B=0.025124,A=1.000000)" 2.0)
  (bind _outactors (Collision|SphereOverlapActors (Transformation|GetWorldLocation (Variables|/Script/Engine.RadialForceActor|GetForceComponent _returnvalue_3)) (Variables|/Script/Engine.RadialForceComponent|GetRadius (Variables|/Script/Engine.RadialForceActor|GetForceComponent _returnvalue_3)) (Variables|Default|GethitTypes) 0))
  (for _array_element _outactors
    (bind _asbp_npc (Utilities|Casting|CastToBP_NPC _array_element)
      (:then
        (Default|GetHitbySneeze _asbp_npc (Transformation|GetActorLocation)))
      (:CastFailed
        (Development|PrintString "Cast Fail"))))
  (bind _asfpsgame_mode (Utilities|Casting|CastToFPSGameMode (Game|GetGameMode))
    (:then
      (Default|EngageinSneezeInterval _asfpsgame_mode)
      (Character|LaunchCharacter (Math|Vector|MakeVector (* (* (Variables|Default|GetRecoilStrength) _x) -1.0) (* (* (Variables|Default|GetRecoilStrength) _y) -1.0) 1e+02) false false)
      (Camera|SetFieldOfView (Variables|Default|GetCamera) 9e+01)
      (Widget|RemovefromParent (Variables|Default|GetSneezeIncomingWidget)))
    (:CastFailed
      (Development|PrintString "Fail Force"))))

(fn AnticipateSneeze
  (Variables|Default|SetAnticipatingSneezeTimer 0.0)
  (Variables|Default|SetAnticipatingSneeze true)
  (bind _returnvalue (UserInterface|CreateWidget "/Game/Blueprints/SneezeIncoming.SneezeIncoming_C"))
  (bind _output_get (Variables|Default|SetSneezeIncomingWidget _returnvalue))
  (UserInterface|Viewport|AddtoViewport _output_get 0))

(fn StartSneezing
  (bind _asfpsgame_mode (Utilities|Casting|CastToFPSGameMode (Game|GetGameMode)))
  (Default|ResetCountingforNextSneezeEvent _asfpsgame_mode)
  (Variables|Default|SetIsSick true))

(fn Dash
  (bind _springarm (Variables|Default|GetSpringArm))
  (bind _returnvalue (Math|Vector|GetForwardVector _springarm))
  (bind _returnvalue_2 (* _returnvalue 1e+02))
  (bind (_x _y) (Math|Vector|BreakVector _returnvalue_2))
  (Character|LaunchCharacter (Math|Vector|MakeVector (* (Variables|Default|GetDashPower) _x) (* (Variables|Default|GetDashPower) _y) 1e+02) false false))