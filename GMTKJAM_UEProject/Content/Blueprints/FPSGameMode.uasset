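; FPS game mode that schedules random bouts of sneezing for the player.
; Tick runs a timer and state machine, rolling for a sneeze at the end of each wait or interval, with odds scaled inversely by the current count.
; A success calls AnticipateSneeze on the player's BP_FPSController character and suspends timing; failure resets to a random long-cycle timer.
; EngageInSneezeInterval, not called here, resumes timing with a random between-sneeze interval.
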(event EventBeginPlay)

(event EventTick
  (params (DeltaSeconds :type Float%20%28single-precision%29))
  (switch Utilities|FlowControl|Switch|SwitchonSneezeState (Variables|Default|GetSneezeState)
    (:NewEnumerator1
      _)
    (:NewEnumerator2
      _))
  (if (> (Variables|Default|GetCurrentTime) (Variables|Default|GetTimeForNextSneeze))
    (bind _sneezehappen (CallFunction|CheckforSneeze (Variables|Default|GetCurrentSneezeCount)))
    (if _sneezehappen
      (CallFunction|SneezeEvent)
      (else
        (CallFunction|ResetCountingforNextSneezeEvent)))
    (else
      (Variables|Default|SetCurrentTime (+ (Variables|Default|GetCurrentTime) DeltaSeconds)))))

(fn ConstructionScript)

(fn ResetCountingforNextSneezeEvent
  (Variables|Default|SetCurrentSneezeCount 0)
  (bind _timeforsneeze (CallFunction|GetRandomSneezeTimer))
  (Variables|Default|SetTimeForNextSneeze _timeforsneeze)
  (Variables|Default|SetCurrentTime 0.0)
  (Variables|Default|SetSneezeState "NewEnumerator1")
  (Development|PrintString "Resetting Sneeze"))

(fn GetRandomSneezeTimer
  (return (Math|Random|RandomFloatinRange (Variables|Default|GetMinimumSneezeTime) (Variables|Default|GetMaximumSneezeTime))))

(fn GetRandomInterval
  (return (Math|Random|RandomFloatinRange (Variables|Default|GetMinimumIntervalTime) (Variables|Default|GetMaximumIntervalTime))))

(fn CheckforSneeze
  (params (SneezeCount :type Integer))
  (if (> SneezeCount 0)
    (return (> (* (Variables|Default|GetInitialSneezeProbability) (/ (Variables|Default|GetSneezeProbabilityFactor) (Math|Conversions|ToFloat(Integer) SneezeCount))) (Math|Random|RandomFloat)))
    (else
      (return (> (Variables|Default|GetInitialSneezeProbability) (Math|Random|RandomFloat))))))

(fn SneezeEvent
  (Math|Integer|IncrementInt (Variables|Default|GetCurrentSneezeCount)
    (:%20%20
      (bind _asbp_fpscontroller (Utilities|Casting|CastToBP_FPSController (Game|GetPlayerCharacter 0)))
      (Default|AnticipateSneeze _asbp_fpscontroller)
      (Variables|Default|SetSneezeState "NewEnumerator3"))))

(fn EngageinSneezeInterval
  (bind _sneezeintervaltime (CallFunction|GetRandomInterval))
  (Variables|Default|SetCurrentTime 0.0)
  (Variables|Default|SetTimeForNextSneeze _sneezeintervaltime)
  (Variables|Default|SetSneezeState "NewEnumerator2"))