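; Scene component that makes its owning actor damageable, charging the player's damage total once when it is knocked loose.
; At start it caches the FPSGameMode and disables physics on the owner's static meshes, which GetHit re-enables.
; Each Tick it polls the attach parent's velocity; the first time this exceeds a threshold, it adds a fee through the game mode and plays a cha-ching sound.
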(event EventBeginPlay
  (bind _asfpsgame_mode (Utilities|Casting|CastToFPSGameMode (Game|GetGameMode)))
  (Variables|Default|SetGameMode _asfpsgame_mode)
  (for _array_element (Actor|GetComponentsByClass (Components|GetOwner) "/Script/Engine.StaticMeshComponent")
    (Physics|SetSimulatePhysics _array_element false)))

(event EventTick
  (params (DeltaSeconds :type Float%20%28single-precision%29))
  (if (not (Variables|Default|GetIsHit))
    (if (> (Math|Vector|VectorLength (Transformation|GetComponentVelocity (Transformation|GetAttachParent))) (Variables|Default|GetVelocityThreshold))
      (Default|AddDamage (Variables|Default|GetGameMode) (Variables|Default|GetDamageFeeOnHit))
      (Audio|PlaySoundatLocation "/Game/Sound/Kachingg.Kachingg" (Transformation|GetActorLocation (Components|GetOwner)) "0, 0, 0" 1.0 1.0 0.0 "/Game/Blueprints/Kachin.Kachin" "/Game/Sound/KachinConcurrency.KachinConcurrency" 0)
      (Variables|Default|SetIsHit true))))

(fn GetHit
  (for _array_element (Actor|GetComponentsByClass (Components|GetOwner) "/Script/Engine.StaticMeshComponent")
    (Physics|SetSimulatePhysics _array_element true)))