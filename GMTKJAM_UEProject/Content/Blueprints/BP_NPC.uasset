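; BP_NPC is a wandering character that gets knocked into a ragdoll when hit by a sneeze.
; On BeginPlay it picks a random skeletal mesh, then roams to nearby navmesh points, pausing after each successful move.
; GetHitBySneeze spawns BP_NPC_Ragdoll with the same mesh, launches it away from the sneeze with a fixed upward kick, and destroys the NPC.
; The wander loop has no failure branch, so a failed move ends it.
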(event Custom|MoveToRandomLocation
  (AI|AIMoveTo self (.RandomLocation (Class|NavigationSystemV1|GetRandomPointinNavigableRadius (Transformation|GetActorLocation) 5e+02 0 0)) 0 5.0 false
    (:OnSuccess
      (Utilities|FlowControl|Delay 3.0)
      (CallFunction|MovetoRandomLocation))))

(event EventBeginPlay
  (bind _output_get (Variables|Default|SetMeshIndex (Math|Float|Truncate (Math|Random|RandomFloatinRange 0.0 6.0))))
  (Class|SkinnedMeshComponent|SetSkeletalMesh (Variables|Character|GetMesh) (Utilities|Array|Get(acopy) (Variables|Default|GetSkeletalMesh) _output_get) true)
  (CallFunction|MovetoRandomLocation))

(fn ConstructionScript)

(fn GetHitbySneeze
  (params (SneezeFromLocation :type Vector))
  (bind _returnvalue (Transformation|GetActorLocation))
  (bind _launchforce (Variables|Default|GetLaunchForce))
  (bind _returnvalue_2 (Math|Vector|GetUnitDirection(Vector) SneezeFromLocation _returnvalue))
  (bind _returnvalue_3 (* _returnvalue_2 _launchforce))
  (bind _returnvalue_4 (Game|SpawnActorfromClass "/Game/Blueprints/BP_NPC_Ragdoll.BP_NPC_Ragdoll_C" (Transformation|GetActorTransform) "Undefined" 0 0))
  (Development|PrintString (Utilities|String|ToString(Vector) _returnvalue_2))
  (Class|SkinnedMeshComponent|SetSkeletalMesh (Variables|/Game/Blueprints/BP_NPC_Ragdoll.BP_NPC_Ragdoll_C|GetSkeletalMesh _returnvalue_4) (Utilities|Array|Get(acopy) (Variables|Default|GetSkeletalMesh) (Variables|Default|GetMeshIndex)) true)
  (Physics|AddImpulse (Variables|/Game/Blueprints/BP_NPC_Ragdoll.BP_NPC_Ragdoll_C|GetSkeletalMesh _returnvalue_4) (Math|Vector|MakeVector (.x _returnvalue_3) (.y _returnvalue_3) 5e+02) "None" false)
  (Actor|DestroyActor))