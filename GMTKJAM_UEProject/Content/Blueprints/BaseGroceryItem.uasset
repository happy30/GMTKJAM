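; BaseGroceryItem is a grocery item actor that charges a one-time damage fee when it gets knocked into motion.
; BeginPlay caches the FPSGameMode, and Tick polls the static mesh's velocity rather than using hit or overlap events.
; When speed first exceeds VelocityThreshold, it passes DamageFeeOnHit to the game mode's AddDamage and sets IsHit to block further charges.
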(event EventBeginPlay
  (bind _asfpsgame_mode (Utilities|Casting|CastToFPSGameMode (Game|GetGameMode)))
  (Variables|Default|SetGameMode _asfpsgame_mode))

(event Collision|EventActorBeginOverlap
  (params (OtherActor :type Actor%20Object%20Reference)))

(event EventTick
  (params (DeltaSeconds :type Float%20%28single-precision%29))
  (if (not (Variables|Default|GetIsHit))
    (if (> (Math|Vector|VectorLength (Transformation|GetComponentVelocity (Variables|Default|GetStaticMesh))) (Variables|Default|GetVelocityThreshold))
      (Default|AddDamage (Variables|Default|GetGameMode) (Variables|Default|GetDamageFeeOnHit))
      (Variables|Default|SetIsHit true))))

(fn ConstructionScript)